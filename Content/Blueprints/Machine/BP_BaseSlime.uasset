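; Slime base machine that shows the type of slime it detects and animates a morph-target hatch with sound.
; On BeginPlay it line-traces along its Arrow for BP_Slime, recolors the base by TypeOfPrinter, and hands the slime its spline and cage settings.
; A scale timeline shrinks the effect plane, swaps in the Area, Damage or Utility material, then reverses.
; Door open and close events drive that plane alongside the morph timeline.
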(event `Anim`
  (`GameplayStatics.PlaySound2D` "/Game/Sound/SFX_SC/Slime_Sc/SC_SFX_Trappe_Ouvre_01.SC_SFX_Trappe_Ouvre_01" 1.0 1.0 0.0 null null)
  (`self.OpenDoor `))

(event `self.ReceiveBeginPlay`
  (`SkeletalMeshComponent.SetMorphTarget` (`self.PR_fermoir_00`) "open" 1.0 true)
  (`self.DetectTypeOfSlime`))

(event `OpenDoor`
  (bind _slimehit (`self.SlimeHit`)
    (:`then`
      (switch `/Game/Blueprints/Enums/Enum_Kit` (`/Game/Blueprints/Machine/BP_Slime.TypeOfPrinter` _slimehit)
        (:`NewEnumerator0`
          (`self.Anim Plane ` "/Game/Assets/Materials/Decals/SlimeDecals/MI_SlimeEffect_Area.MI_SlimeEffect_Area")
          (bind (_direction _newtrack_0) (`Timeline|Timeline` :!via `PlayFromStart` :!label _label)
            (:`Update`
              (`SkeletalMeshComponent.SetMorphTarget` (`self.PR_fermoir_00`) "open" (`KismetMathLibrary.Lerp` 1.0 0.0 _newtrack_0) false))))
        (:`NewEnumerator1`
          (`self.Anim Plane ` "/Game/Assets/Materials/Decals/SlimeDecals/MI_SlimeEffect_Damage.MI_SlimeEffect_Damage")
          (goto _label :!via `PlayFromStart`))
        (:`NewEnumerator2`
          (`self.Anim Plane ` "/Game/Assets/Materials/Decals/SlimeDecals/MI_SlimeEffect_Utility.MI_SlimeEffect_Utility")
          (goto _label :!via `PlayFromStart`))))
    (:`else`)))

(event `CloseDoort`
  (`self.Reverse Anim Plane`)
  (goto _label :!via `ReverseFromEnd`))

(event `DetectTypeOfSlime`
  (bind _slimehit (`self.SlimeHit`))
  (bind _pr_socleslime_00 (`self.PR_socleSlime_00`))
  (bind _returnvalue (`SceneComponent.K2_GetComponentLocation` (`self.Arrow`)))
  (`GameplayStatics.PlaySound2D` "/Game/Sound/SFX_SC/Slime_Sc/SC_SFX_Trappe_Ferme_01.SC_SFX_Trappe_Ferme_01" 1.0 1.0 0.0 null null)
  ;[1 1 1] Comment
  (bind _outhits (`KismetSystemLibrary.LineTraceMulti` _returnvalue (+ _returnvalue (* (`SceneComponent.GetForwardVector` (`self.Arrow`)) 5000.0)) "TraceTypeQuery1"))
  (for _array_element _outhits
    (bind _asbp_slime (cast `/Game/Blueprints/Machine/BP_Slime` (`.HitActor` (`GameplayStatics.BreakHitResult` _array_element))))
    (bind _output_get (set `self.SlimeHit` _asbp_slime))
    (switch `/Game/Blueprints/Enums/Enum_Kit` (`/Game/Blueprints/Machine/BP_Slime.TypeOfPrinter` _output_get)
      (:`NewEnumerator0`
        (`PrimitiveComponent.SetMaterial` _pr_socleslime_00 2 "/Game/Assets/Assembleur/Mat/lcd_Red.lcd_Red")
        (`PrimitiveComponent.SetMaterial` _pr_socleslime_00 1 "/Game/Assets/Assembleur/Mat/MI_metal_Red.MI_metal_Red")
        (`PrimitiveComponent.SetMaterial` _pr_socleslime_00 0 "/Game/Assets/Assembleur/Mat/Led_Red.Led_Red")
        (`self.Anim Plane ` "/Game/Assets/Materials/Decals/SlimeDecals/MI_SlimeEffect_Area.MI_SlimeEffect_Area" true))
      (:`NewEnumerator1`
        (`PrimitiveComponent.SetMaterial` _pr_socleslime_00 2 "/Game/Assets/Assembleur/Mat/lcd_Green.lcd_Green")
        (`PrimitiveComponent.SetMaterial` _pr_socleslime_00 1 "/Game/Assets/Assembleur/Mat/M_metal.M_metal")
        (`PrimitiveComponent.SetMaterial` _pr_socleslime_00 0 "/Game/Assets/Assembleur/Mat/Led_Green.Led_Green")
        (`self.Anim Plane ` "/Game/Assets/Materials/Decals/SlimeDecals/MI_SlimeEffect_Damage.MI_SlimeEffect_Damage" true))
      (:`NewEnumerator2`
        (`PrimitiveComponent.SetMaterial` _pr_socleslime_00 2 "/Game/Assets/Assembleur/Mat/lcd_Blue.lcd_Blue")
        (`PrimitiveComponent.SetMaterial` _pr_socleslime_00 1 "/Game/Assets/Assembleur/Mat/MI_metal_Blue.MI_metal_Blue")
        (`PrimitiveComponent.SetMaterial` _pr_socleslime_00 0 "/Game/Assets/Assembleur/Mat/Led_Blue.Led_Blue")
        (`self.Anim Plane ` "/Game/Assets/Materials/Decals/SlimeDecals/MI_SlimeEffect_Utility.MI_SlimeEffect_Utility" true)))
    (set `/Game/Blueprints/Machine/BP_Slime.IsSpline` (`self.Spline`) (`self.SlimeHit`))
    (if (`self.HasCage`)
      (set `/Game/Blueprints/Machine/BP_Slime.cage` (`self.WhatCage`) _slimehit)
      (break)
      (else
        (set `/Game/Blueprints/Machine/BP_Slime.cage` null _slimehit)))))

(event `Anim Plane`
  (params (Material :type "MaterialInterface Object Reference") (Condition :type Boolean))
  (set `self.b_reverse_anim` false)
  (bind (_direction _alpha) (`Timeline|TL_Plane_Scale` :!via `PlayFromStart` :!label _label_2)
    (:`Update`
      (bind _returnvalue (`KismetMathLibrary.Lerp` 1.75 0.0 _alpha))
      (`SceneComponent.SetRelativeScale3D` (`self.Plane`) (`KismetMathLibrary.MakeVector` _returnvalue _returnvalue 1.75)))
    (:`Finished`
      (if Condition
        (if (not (`self.b_reverse_anim`))
          (`PrimitiveComponent.SetMaterial` (`self.Plane`) 0 Material)
          (`self.Reverse Anim Plane`))))))

(event `Reverse Anim Plane`
  (set `self.b_reverse_anim` true)
  (goto _label_2 :!via `ReverseFromEnd`))

(fn `NewFunction`
  (switch `/Game/Blueprints/Enums/Enum_Kit` "NewEnumerator2"))

(fn `UserConstructionScript`)