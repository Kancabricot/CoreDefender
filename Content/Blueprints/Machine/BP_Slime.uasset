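; Slime machine that eats scraps dropped into its trigger and spits out turret kits of its color type, with golden scraps yielding several.
; Overlap banks scrap value and plays eating effects; CreateAddons spends it, spawns kits, then starts sleep.
; Sleep lowers the slime and runs a timer-driven bar until it wakes and rises, with BP_GestionSlime handling position shuffles.
; A dynamic eye material swaps flipbook faces per type, and widgets support the tutorial.
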(event `self.ReceiveBeginPlay`
  (bind _niagara_goldenscrap (`self.Niagara_GoldenScrap`))
  ;[1 1 1] BeginPlay
  (`SceneComponent.SetVisibility` (`self.widgetThrow`) false false)
  (bind _returnvalue (`GameplayStatics.GetActorOfClass` "/Game/Blueprints/Machine/BP_GestionSlime.BP_GestionSlime_C"))
  (set `self.GestionMachine` _returnvalue)
  (bind _returnvalue_2 (`PrimitiveComponent.CreateDynamicMaterialInstance` (`self.Rebl_Chewing_01`) 1 (`self.EyesMat`) "None"))
  (set `self.DynamicM` _returnvalue_2)
  (set `self.FirstRotation` (`SceneComponent.K2_GetComponentRotation` (`self.Rebl_Chewing_01`)))
  ;;[1 1 1] Widgets Ref
  (bind _aswg_slime_sleeping (cast `/Game/Blueprints/Widgets/WG_SlimeSleeping` (`WidgetComponent.GetWidget` (`self.WidgetSleep`))))
  (bind _output_get (set `self.As WG Slime Sleeping` _aswg_slime_sleeping))
  (`Widget.SetVisibility` _output_get "Hidden")
  (`SceneComponent.SetVisibility` (`self.widgetScrap`) false false)
  (bind _aswg_circle (cast `/Game/Blueprints/Widgets/WG_Circle` (`WidgetComponent.GetWidget` (`self.Widget_Circle`))))
  (set `self.As WG Circle` _aswg_circle)
  (`ActorComponent.Deactivate` _niagara_goldenscrap)
  (`SceneComponent.SetVisibility` _niagara_goldenscrap false false))

(event `Show Widgets`
  ;[1 1 1] Scrap Widgets Tuto
  (if (not (or (`self.IsCrafting`) (`self.b_Tuto_is_Inactactive`) (`self.isSleeping`)))
    (`/Game/Blueprints/Widgets/WG_Circle.Play Circle Animation` (`self.As WG Circle`))
    (`SceneComponent.SetVisibility` (`self.widgetScrap`) true false)))

(event `Hide Widgets`
  ;[1 1 1] Scrap Widgets Tuto
  (if (not (or (`self.IsCrafting`) (`self.b_Tuto_is_Inactactive`) (`self.isSleeping`)))
    (`SceneComponent.SetVisibility` (`self.widgetScrap`) false false)))

(event `SleepPhase`
  (bind _niagara (`self.Niagara`))
  ;[1 1 1] Sleep and wake up
  (`self.TutorialmanagerRef`
    (:`then`
      (`self.Hide Widgets`))
    (:`else`
      _))
  (set `self.isSleeping` true)
  (set `self.IsCrafting` false)
  (`KismetSystemLibrary.Delay` 1.0)
  (`Widget.SetVisibility` (`self.As WG Slime Sleeping`) "Visible")
  (`ActorComponent.Activate` _niagara false)
  (`SceneComponent.SetVisibility` _niagara true false)
  (bind _returnvalue (`KismetSystemLibrary.K2_SetTimerDelegate` (delegate `TimerSleep`) (`self.TimerDuration`) true -1.0))
  (set `self.DelayTimer` _returnvalue)
  (`self.Anim` false)
  (`/Game/Blueprints/Machine/BP_BaseSlime.OpenDoor ` (`self.Base`)))

(event `TimerSleep`
  ;[1 1 1] Sleep and wake up
  (bind _output_get (set `self.ActuSleepDuration` (+ (`self.ActuSleepDuration`) 1.0)))
  (`/Game/Blueprints/Widgets/WG_SlimeSleeping.Set Slime Sleep Bar` (`self.As WG Slime Sleeping`) _output_get (`self.MaxSleepDuration`))
  (if (>= (`self.ActuSleepDuration`) (`self.MaxSleepDuration`))
    (`self.Wakeup`)
    (`self.ReversiAim` (.z (.location (`|GetArrayItem` (`/Game/Blueprints/Machine/BP_GestionSlime.TabTest` (`self.GestionMachine`))))))))

(event `Wakeup`
  (bind _niagara (`self.Niagara`))
  ;[1 1 1] Sleep and wake up
  (set `self.CanEat` true)
  (`ActorComponent.Deactivate` _niagara)
  (`SceneComponent.SetVisibility` _niagara false false)
  (set `self.isSleeping` false)
  (`Widget.SetVisibility` (`self.As WG Slime Sleeping`) "Hidden")
  (bind _output_get (set `self.ActuSleepDuration` 0.0))
  (`/Game/Blueprints/Widgets/WG_SlimeSleeping.Set Slime Sleep Bar` (`self.As WG Slime Sleeping`) _output_get (`self.MaxSleepDuration`))
  (`KismetSystemLibrary.K2_PauseTimerHandle` (`self.DelayTimer`))
  (set `self.TimerDuration` 1.0)
  (`/Game/Blueprints/Widgets/WG_SlimeSleeping.ChangeBack` (`self.As WG Slime Sleeping`)))

(event `PlayAnime`
  (params (WhatFace :type Integer))
  (bind (_nbframe _face) (`self.GetGoodFace` WhatFace))
  ;[1 1 1] Animation
  ;;[1 1 1] PlayFaceAnime
  (`self.ChangeFacialAnim` _nbframe _face))

(event `Anim`
  (params (Shuffle :type Boolean))
  (bind (_returnvalue_x _returnvalue_y _returnvalue_z) (`KismetMathLibrary.BreakVector` (`self.K2_GetActorLocation`)))
  ;[1 1 1] Animation
  (if (not (`self.IsInGround`))
    (bind (_direction _newtrack_0) (`Timeline|Timeline` :!via `PlayFromStart`)
      (:`Update`
        (`self.K2_SetActorLocation` (`KismetMathLibrary.MakeVector` _returnvalue_x _returnvalue_y (`KismetMathLibrary.Lerp` _returnvalue_z (+ _returnvalue_z -10.0) _newtrack_0))))
      (:`Finished`
        (set `self.IsInGround` true)
        (if (`self.b_IsTuto`)
          (set `self.b_Tuto_is_Inactactive` true)
          (elif Shuffle
            (`self.Suflle`)))))))

(event `Suflle`
  ;[1 1 1] Animation
  (`/Game/Blueprints/Machine/BP_GestionSlime.ShuffleMachine` (`self.GestionMachine`)))

(event `Revien`
  (`KismetSystemLibrary.K2_PauseTimerHandle` (`self.DelayTimer`))
  (set `self.TimerDuration` 1.0)
  (`/Game/Blueprints/Widgets/WG_SlimeSleeping.ChangeBack` (`self.As WG Slime Sleeping`))
  (`self.SleepPhase`))

(event `ReversiAim`
  (params (`Z Transform` :type "Float (double-precision)") (shuflle :type Boolean) (`INDEX TAB` :type Integer))
  (bind (_returnvalue_x _returnvalue_y _returnvalue_z) (`KismetMathLibrary.BreakVector` (`self.K2_GetActorLocation`)))
  ;[1 1 1] Animation
  (if (`self.isSleeping`)
    (`self.Anim` false)
    (else
      (bind (_direction _newtrack_0) (`Timeline|Timeline_0` :!via `PlayFromStart`)
        (:`Update`
          (`self.K2_SetActorLocation` (`KismetMathLibrary.MakeVector` _returnvalue_x _returnvalue_y (`KismetMathLibrary.Lerp` _returnvalue_z `Z Transform` _newtrack_0))))
        (:`Finished`
          (set `self.IsInGround` false)
          (if (`self.b_IsTuto`)
            (set `self.b_Tuto_is_Inactactive` false)))))))

(event `self.gIVEbOX.OnComponentBeginOverlap`
  (params (OverlappedComponent :type "PrimitiveComponent Object Reference") (OtherActor :type "Actor Object Reference") (OtherComp :type "PrimitiveComponent Object Reference") (OtherBodyIndex :type Integer) (bFromSweep :type Boolean) (SweepResult :type "HitResult Structure (by ref)"))
  (bind _niagara_goldenscrap (`self.Niagara_GoldenScrap`))
  (bind _as_bp_scrap (`self.As BP Scrap`))
  (bind (_returnvalue_x _returnvalue_y _returnvalue_z) (`KismetMathLibrary.BreakVector` (`SceneComponent.K2_GetComponentLocation` (`self.MiamVFX_Scene`))))
  (bind (_returnvalue_x_2 _returnvalue_y_2 _returnvalue_z_2) (`KismetMathLibrary.BreakVector` (`SceneComponent.K2_GetComponentLocation` (`self.Rebl_Chewing_01`))))
  (bind (_returnvalue_x_3 _returnvalue_y_3) (`KismetMathLibrary.BreakVector` (`KismetMathLibrary.VInterpTo` (`self.K2_GetActorLocation` (`self.As BP Scrap`)) (`SceneComponent.K2_GetComponentLocation` (`self.Rebl_Chewing_01`)) (`GameplayStatics.GetWorldDeltaSeconds`) 10.0)))
  (bind _returnvalue (`KismetMathLibrary.MakeVector` _returnvalue_x _returnvalue_y (- _returnvalue_z 75.0)))
  ;[1 1 1] When box is given
  (if (and (`self.CanEat`) (not (`self.b_Tuto_is_Inactactive`)))
    (`self.TutorialmanagerRef`
      (:`then`
        (`self.Hide Widgets`))
      (:`else`
        _))
    (bind _cage (`self.cage`)
      (:`then`
        (if (not (`/Game/Blueprints/LevelPrototyping/BP_LaserCage.GateActivated` _cage))
          (bind _asbp_scrap (cast `/Game/Blueprints/Enemie/Blueprint/BP_Scrap` OtherActor :!label _label))
          (set `/Game/Blueprints/Enemie/Blueprint/BP_Scrap.b_cantBeGrab` true _asbp_scrap)
          (if (`/Game/Blueprints/Enemie/Blueprint/BP_Scrap.Grabable` _asbp_scrap)
            (set `self.As BP Scrap` _asbp_scrap)
            (cast `/Game/Blueprints/Enemie/Blueprint/BP_GoldenScrap` (`self.As BP Scrap`)
              (:`then`
                (`self.SetActorEnableCollision` OtherActor false)
                (`ActorComponent.Activate` _niagara_goldenscrap false)
                (`SceneComponent.SetVisibility` _niagara_goldenscrap true false))
              (:`CastFailed`
                _))
            (bind _spline_ref (`/Game/Blueprints/Enemie/Blueprint/BP_Scrap.Spline Ref` _asbp_scrap)
              (:`then`
                (`self.K2_DestroyActor` _spline_ref))
              (:`else`
                _))
            (set `self.NbScrap` (+ (`/Game/Blueprints/Enemie/Blueprint/BP_Scrap.Value` (`self.As BP Scrap`)) (`self.NbScrap`)))
            (`|ExecutionSequence`
              (:`then_0`
                (`PrimitiveComponent.SetCollisionEnabled` (`/Game/Blueprints/Enemie/Blueprint/BP_Scrap.StaticMesh1` _as_bp_scrap) "NoCollision")
                (`PrimitiveComponent.SetCollisionEnabled` (`/Game/Blueprints/Enemie/Blueprint/BP_Scrap.Box` _as_bp_scrap) "NoCollision")
                (`self.SetActorEnableCollision` _as_bp_scrap false)
                (`Timeline|GoTo` :!via `PlayFromStart`
                  (:`Update`
                    (`self.K2_SetActorLocation` (`self.As BP Scrap`) (`KismetMathLibrary.MakeVector` _returnvalue_x_3 _returnvalue_y_3 _returnvalue_z_2) false false))
                  (:`Finished`
                    (`/Game/Blueprints/Enemie/Blueprint/BP_Scrap.FunctionDestroyActor` (`self.As BP Scrap`)))))
              (:`then_1`
                (set `self.CanEat` false)
                (set `self.GrabScrap` true)
                (set `self.IsCrafting` true)
                (cast `/Game/Blueprints/Enemie/Blueprint/BP_GoldenScrap` (`self.As BP Scrap`)
                  (:`then`
                    (bind _returnvalue_2 (`NiagaraFunctionLibrary.SpawnSystemAtLocation` "/Game/VFXToLoad/NS_EatingEffect_GoldenScrap.NS_EatingEffect_GoldenScrap" _returnvalue (struct) (1.0 1.0 1.0) false))
                    (`KismetSystemLibrary.Delay` (`self.CraftingDuration`))
                    (set `self.IsCrafting` false)
                    (`ActorComponent.K2_DestroyComponent` _returnvalue_2))
                  (:`CastFailed`
                    (bind _returnvalue_3 (`NiagaraFunctionLibrary.SpawnSystemAtLocation` "/Game/VFXToLoad/NS_EatingEffect.NS_EatingEffect" _returnvalue (struct) (1.0 1.0 1.0) false))
                    (`KismetSystemLibrary.Delay` (`self.CraftingDuration`))
                    (set `self.IsCrafting` false)
                    (`ActorComponent.K2_DestroyComponent` _returnvalue_3))))))))
      (:`else`
        (goto _label)))))

(event `CreateAddons`
  (bind _gestionmachine (`self.GestionMachine`))
  (bind _niagara_goldenscrap (`self.Niagara_GoldenScrap`))
  (bind _niagara_goldenscrap_2 (`self.Niagara_GoldenScrap`))
  (bind _returnvalue (`SceneComponent.K2_GetComponentLocation` (`self.Scene`)))
  ;[1 1 1] CreateAddons event
  (set `self.NbScrap` (- (`self.NbScrap`) (`self.ScrapNeeded`) 0))
  (`NiagaraFunctionLibrary.SpawnSystemAtLocation` "/Game/VFX/VFX/Distributeur/StarSuccess/NS_StarSuccess.NS_StarSuccess" _returnvalue)
  (cast `/Game/Blueprints/Enemie/Blueprint/BP_GoldenScrap` (`self.As BP Scrap`)
    (:`then`
      (`ActorComponent.Activate` _niagara_goldenscrap_2 false)
      (`SceneComponent.SetVisibility` _niagara_goldenscrap_2 true false)
      (bind _index (`/Game/Blueprints/Macro/ML_Macro.ForLoopWithDelay` 0 2 2.0 -2.0)
        (:`LoopBody`
          (bind _returnvalue_2 (`|SpawnActorFromClass` "/Game/Blueprints/Turret/Blueprint/BP_TurretKit.BP_TurretKit_C" (`KismetMathLibrary.MakeTransform` _returnvalue) "Undefined" "MultiplyWithRoot" null (`KismetMathLibrary.RandomIntegerInRange` -2147483648 2147483647) (`self.TypeOfPrinter`) null :!label _label_2))
          (set `/Game/Blueprints/Player/Player/BP_Throw.ActorTarget` _returnvalue_2 (`self.IsSpline`))
          (if (`self.b_Give_TutoManager_Ref_`)
            (set `/Game/Blueprints/Turret/Blueprint/BP_TurretKit.BP_TutorialManager` (`self.TutorialmanagerRef`) _returnvalue_2)))
        (:`Complete`
          (`ActorComponent.Deactivate` _niagara_goldenscrap)
          (`SceneComponent.SetVisibility` _niagara_goldenscrap false false)
          (`self.SleepPhase` :!label _label_3)
          (`/Engine/EditorBlueprintResources/StandardMacros.IsValid` _gestionmachine
            (:`Is Valid`
              (if (`/Game/Blueprints/Machine/BP_GestionSlime.b_NeedToShuffle` _gestionmachine)
                (`KismetSystemLibrary.Delay` 2.0)
                (`/Game/Blueprints/Machine/BP_GestionSlime.Shuffle` _gestionmachine)))
            (:`Is Not Valid`
              _))
          (bind _tutorialmanagerref (`self.TutorialmanagerRef`)
            (:`then`
              (`/Game/Blueprints/Tutorial/BP_TutorialManager.Slime` _tutorialmanagerref))
            (:`else`)))))
    (:`CastFailed`
      (`|ExecutionSequence`
        (:`then_0`
          (goto _label_2))
        (:`then_1`
          (goto _label_3))))))

(fn `ChangeFacialAnim`
  (params (nbFrame :type "Float (single-precision)") (Face :type "Texture Object Reference"))
  (`MaterialInstanceDynamic.SetScalarParameterValue` (`self.DynamicM`) "Nombre D'image" nbFrame)
  (`MaterialInstanceDynamic.SetTextureParameterValue` (`self.DynamicM`) "Texture" Face))

(fn `GetGoodFace`
  (params (WhatFace :type Integer))
  (returns (nbFrame :type "Float (double-precision)") (Face :type "Texture Object Reference"))
  (bind _face (break `/Game/Blueprints/Machine/FaceStructure` (`BlueprintMapLibrary.Map_Find` (`self.MapsTypeFace`) (`self.TypeOfPrinter`))))
  (bind _keys (`BlueprintMapLibrary.Map_Keys` _face))
  (bind _output (`|GetArrayItem` _keys WhatFace))
  (return (`BlueprintMapLibrary.Map_Find` _face _output) _output))

(fn `Spit Out Scraps`
  (bind _returnvalue (- (`self.NbScrap`) (`self.ScrapNeeded`)))
  (if (<= _returnvalue 3)
    (bind _returnvalue_2 (`|SpawnActorFromClass` "/Game/Blueprints/Enemie/Blueprint/BP_Scrap.BP_Scrap_C" (`KismetMathLibrary.MakeTransform` (`SceneComponent.K2_GetComponentLocation` (`self.Scrap Spawn`))) "Undefined" "MultiplyWithRoot" null _returnvalue null))
    (set `/Game/Blueprints/Enemie/Blueprint/BP_Scrap.Value` _returnvalue _returnvalue_2)
    (`PrimitiveComponent.SetPhysicsLinearVelocity` (`/Game/Blueprints/Enemie/Blueprint/BP_Scrap.StaticMesh` _returnvalue_2) (`self.Impulse Scrap`) false "None")))

(fn `UserConstructionScript`
  (bind _rebl_chewing_01 (`self.Rebl_Chewing_01`))
  (bind _rebl_chewing_01_2 (`self.Rebl_Chewing_01`))
  (bind _rebl_chewing_01_3 (`self.Rebl_Chewing_01`))
  (switch `/Game/Blueprints/Enums/Enum_Kit` (`self.TypeOfPrinter`)
    (:`NewEnumerator0`
      (`PrimitiveComponent.SetMaterial` _rebl_chewing_01_2 0 "/Game/Assets/Assembleur/Mat/Slime_Inst_Red.Slime_Inst_Red")
      (`SkeletalMeshComponent.SetSkeletalMeshAsset` _rebl_chewing_01_2 "/Game/Assets/Assembleur/Slime/Slime_v4.Slime_v4")
      (set `self.EyesMat` "/Game/Assets/Assembleur/Mat/M_FaceSlime_red.M_FaceSlime_red"))
    (:`NewEnumerator1`
      (`SkeletalMeshComponent.SetSkeletalMeshAsset` _rebl_chewing_01 "/Game/Assets/Assembleur/Slime/Slime_v4.Slime_v4")
      (`PrimitiveComponent.SetMaterial` _rebl_chewing_01 0 "/Game/Assets/Assembleur/Mat/Slime_Inst_green.Slime_Inst_green")
      (set `self.EyesMat` "/Game/Assets/Assembleur/Mat/M_FaceSlime_green.M_FaceSlime_green"))
    (:`NewEnumerator2`
      (`PrimitiveComponent.SetMaterial` _rebl_chewing_01_3 0 "/Game/Assets/Assembleur/Mat/Slime_Inst_Blue.Slime_Inst_Blue")
      (`SkeletalMeshComponent.SetSkeletalMeshAsset` _rebl_chewing_01_3 "/Game/Assets/Assembleur/Slime/Slime_v4.Slime_v4")
      (set `self.EyesMat` "/Game/Assets/Assembleur/Mat/M_FaceSlime_blue.M_FaceSlime_blue")))
  (`PrimitiveComponent.SetMaterial` (`self.Rebl_Chewing_01`) 1 (`self.EyesMat`)))